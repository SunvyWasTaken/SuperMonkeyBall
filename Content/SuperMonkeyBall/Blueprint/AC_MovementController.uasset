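; Movement component for a Super Monkey Ball-style ball that simulates velocity itself and moves the owner with a swept offset each tick.
; Each tick a predictive downward sphere trace sets Grounded and the ground normal, then gravity is applied and projected onto the ground plane.
; Move adds camera-relative force along the slope while grounded, or friction without input.
; Older FCalcule, FMoveForward and FMoveRight functions are unfinished, unused leftovers.
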(event `self.ReceiveBeginPlay`
  ;[0.1144 0.1144 0.1144] Get Owner SphereCollider
  (set `self.SphereCollider` (`Actor.GetComponentByClass` (`self.GetOwner`) "/Script/Engine.SphereComponent")))

(event `self.ReceiveTick`
  (params (DeltaSeconds :type "Float (single-precision)"))
  ;[0.1144 0.1144 0.1144] Upadate Position From Velocity
  (`self.IsGrounded`)
  (`self.ApplyGravity`)
  (`Actor.K2_AddActorWorldOffset` (`self.GetOwner`) (* DeltaSeconds (`self.Velocity`)) true false))

(fn `AddForce`
  (params (Force :type "Vector Structure"))
  (set `self.Velocity` (+ Force (`self.Velocity`))))

(fn `ApplyGravity`
  ;[0.1144 0.1144 0.1144] Apply Gravity
  (set `self.Velocity` (- (`self.Velocity`) (`KismetMathLibrary.MakeVector` 0.0 0.0 (* (`self.Gravity`) (`self.Mass`) (`GameplayStatics.GetWorldDeltaSeconds`)))))
  (if (`self.Grounded`)
    ;[0.1144 0.1144 0.1144] Apply Ground Normal When Grounded
    (set `self.Velocity` (`KismetMathLibrary.ProjectVectorOnToPlane` (`self.Velocity`) (`self.GroundNormal`)))))

(fn `F_CalculeGravity`
  (locals (OutHit :type "HitResult Structure") (Radius :type "Float (single-precision)" :default 0.0))
  (bind _returnvalue (`self.GetOwner`))
  (bind _returnvalue_2 (`Actor.K2_GetActorLocation` (`self.GetOwner`)))
  (if (`self.IsActive`)
    (set `local.Radius` (`KismetMathLibrary.BreakVector3f` (`.BoxExtent` (`Actor.GetActorBounds` _returnvalue true false))))
    ;[1 1 1] POur le Debug
    (`KismetSystemLibrary.PrintString` (`KismetStringLibrary.Concat_StrStr` "Fall Velocity : " (`KismetStringLibrary.Conv_DoubleToString` 0.0)) true true (struct :`R` 1.0 :`G` 0.68913 :`A` 1.0) (`GameplayStatics.GetWorldDeltaSeconds`))
    (bind (_outhit _returnvalue_3) (`KismetSystemLibrary.SphereTraceSingle` :`Start` _returnvalue_2 :`End` (- (+ _returnvalue_2 (0.0 0.0 0.0)) (+ (* (`Actor.GetActorUpVector` _returnvalue) -1.0 (0.0 0.0 0.0)) (0.0 0.0 25.0))) :`Radius` (`local.Radius`) :`TraceChannel` "TraceTypeQuery1" :`DrawDebugType` "ForOneFrame"))
    (set `local.OutHit` _outhit)
    (else
      (return))))

(fn `F_CalculeMovement`
  ;[0.8222 0 1] A revoir parce que jamais encore fait de truc avec la friction
  (if (<= (`KismetMathLibrary.VSize` (`KismetMathLibrary.Normal` (+ (0.0 0.0 0.0) (0.0 0.0 0.0)))) 0.0)
    _))

(fn `F_MoveForward`
  (params (Axis :type "Float (double-precision)"))
  (return))

(fn `F_MoveRight`
  (params (Axis :type "Float (double-precision)"))
  (return))

(fn `GetForwardVector`
  (params (RightVector :type "Vector Structure"))
  (returns (Forward :type "Vector Structure"))
  (return (`KismetMathLibrary.Cross_VectorVector` RightVector (`self.GroundNormal`))))

(fn `IsGrounded`
  (bind _returnvalue (+ (`Actor.K2_GetActorLocation` (`self.GetOwner`)) (* (`self.Velocity`) (`GameplayStatics.GetWorldDeltaSeconds`))))
  (bind (_outhit _returnvalue_2) (`KismetSystemLibrary.SphereTraceSingle` :`Start` _returnvalue :`End` (+ _returnvalue (`KismetMathLibrary.MakeVector` 0.0 0.0 -1.5)) :`Radius` (`self.GroundCheckRadius`) :`TraceChannel` "TraceTypeQuery2" :`DrawDebugType` "ForOneFrame"))
  (set `self.GroundNormal` (`.ImpactNormal` (`GameplayStatics.BreakHitResult` _outhit)))
  (set `self.Grounded` _returnvalue_2))

(fn `Move`
  (params (HorizontalInput :type "Float (double-precision)") (VerticalInput :type "Float (double-precision)") (CameraRight :type "Vector Structure"))
  (bind _velocity (`self.Velocity`))
  (bind _cameraright (`local.CameraRight`))
  (bind _moveforce (`self.MoveForce`))
  (if (`self.Grounded`)
    (if (and (== (`local.HorizontalInput`) 0.0) (== (`local.VerticalInput`) 0.0) (!= (`KismetMathLibrary.VSize` (`self.Velocity`)) 0.0))
      ;[0.1144 0.1144 0.1144] Apply Friction
      (if (> (`KismetMathLibrary.VSize` _velocity) (`self.ZeroThresholdFriction`))
        (set `self.Velocity` (- _velocity (* _velocity (`self.FrictionForce`) (`GameplayStatics.GetWorldDeltaSeconds`))))
        (else
          (set `self.Velocity` (0.0 0.0 0.0))))
      (else
        ;[0.1144 0.1144 0.1144] Add Movement Force
        (`self.AddForce` (* (+ (* (`local.HorizontalInput`) _cameraright _moveforce) (* (`local.VerticalInput`) (`self.GetForwardVector` _cameraright) _moveforce)) (`GameplayStatics.GetWorldDeltaSeconds`)))))))