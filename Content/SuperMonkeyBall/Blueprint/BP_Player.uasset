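; Player pawn for the Super Monkey Ball project that turns Enhanced Input into movement requests.
; On BeginPlay it adds the DefaultInput mapping context to its player controller's local subsystem.
; IA_Move Triggered and Completed share one path, passing X and Y to the ACMonkeyMovement component's FMoveRight and FMoveForward.
; That path also prints the input axis on screen for debugging.
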(event `self.ReceiveBeginPlay`
  (bind _asplayer_controller (cast `PlayerController` (`self.GetController`)))
  (bind _returnvalue (pcsubsystem `EnhancedInputLocalPlayerSubsystem` _asplayer_controller))
  (`/Engine/EditorBlueprintResources/StandardMacros.IsValid` _returnvalue
    (:`Is Valid`
      (`EnhancedInputSubsystemInterface.AddMappingContext` _returnvalue (`self.DefaultInput`) 0 (struct)))))

(event `EnhancedInput|/Game/SuperMonkeyBall/Input/IA_Move`
  (params (ActionValue :type "Vector2D Structure") (ElapsedSeconds :type "Float (double-precision)") (TriggeredSeconds :type "Float (double-precision)") (InputAction :type "InputAction Object Reference" :default "/Game/SuperMonkeyBall/Input/IA_Move.IA_Move"))
  (bind (_x _y) (`KismetMathLibrary.BreakVector2D` ActionValue))
  (:`Triggered`
    ;[0 0.7993 1] Debug Input Axis
    (`KismetSystemLibrary.PrintString` (`KismetStringLibrary.Concat_StrStr` "Input axis : " (`KismetStringLibrary.Conv_Vector2dToString` ActionValue)) true true (struct :`R` 1.0 :`B` 0.025663 :`A` 1.0) (`GameplayStatics.GetWorldDeltaSeconds`) :!label _label)
    (`/Game/SuperMonkeyBall/Blueprint/AC_MonkeyMovement.F_MoveRight` (`self.AC_MonkeyMovement`) _x)
    (`/Game/SuperMonkeyBall/Blueprint/AC_MonkeyMovement.F_MoveForward` (`self.AC_MonkeyMovement`) _y))
  (:`Completed`
    (goto _label)))

(fn `UserConstructionScript`)