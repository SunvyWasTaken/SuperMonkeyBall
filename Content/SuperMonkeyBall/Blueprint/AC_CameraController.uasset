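; Camera controller component for a Super Monkey Ball-style game, which also handles player move input.
; On BeginPlay it adds the input mapping context and caches the owner's camera, spring arm and AC_MovementController.
; Each Tick it passes IA_Move input and the spring arm's right vector to the movement controller.
; It then eases the spring arm toward the velocity's direction, pitched down, with input-driven roll and pitch tilt mimicking a tilting stage.
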(event `self.ReceiveBeginPlay`
  ;[0.1144 0.1144 0.1144] Create SpringArm, Camera and Get MovementController
  (bind _asplayer_controller (cast `PlayerController` (`Pawn.GetController` (`GameplayStatics.GetPlayerPawn` 0))))
  (bind _returnvalue (pcsubsystem `EnhancedInputLocalPlayerSubsystem` _asplayer_controller))
  (`/Engine/EditorBlueprintResources/StandardMacros.IsValid` _returnvalue
    (:`Is Valid`
      (`EnhancedInputSubsystemInterface.AddMappingContext` _returnvalue "/Game/SuperMonkeyBall/Input/IMC_Test.IMC_Test" 0 (struct))
      (`self.GetCamera`)
      (set `self.MovementController` (`Actor.GetComponentByClass` (`self.GetOwner`) "/Game/SuperMonkeyBall/Blueprint/AC_MovementController.AC_MovementController_C"))
      (set `self.SpringArmRef` (`Actor.GetComponentByClass` (`self.GetOwner`) "/Script/Engine.SpringArmComponent")))))

(event `EnhancedInput|/Game/SuperMonkeyBall/Input/IA_Move`
  (params (ActionValue :type "Vector2D Structure") (ElapsedSeconds :type "Float (double-precision)") (TriggeredSeconds :type "Float (double-precision)") (InputAction :type "InputAction Object Reference" :default "/Game/SuperMonkeyBall/Input/IA_Move.IA_Move"))
  (bind (_x _y) (`KismetMathLibrary.BreakVector2D` (`KismetMathLibrary.Normal2D` ActionValue)))
  ;[0.1144 0.1144 0.1144] Get Inputs Value
  (:`Triggered`
    (set `self.InputX` _x)
    (set `self.InputY` _y))
  (:`Canceled`
    (set `self.InputX` 0.0 :!label _label)
    (set `self.InputY` 0.0))
  (:`Completed`
    (goto _label)))

(event `self.ReceiveTick`
  (params (DeltaSeconds :type "Float (single-precision)"))
  (bind _springarmref (`self.SpringArmRef`))
  (bind _roll (.roll (`KismetMathLibrary.Conv_VectorToRotator` (`/Game/SuperMonkeyBall/Blueprint/AC_MovementController.Velocity` (`self.MovementController`)))))
  (bind _returnvalue (- (.pitch (`KismetMathLibrary.Conv_VectorToRotator` (`/Game/SuperMonkeyBall/Blueprint/AC_MovementController.Velocity` (`self.MovementController`)))) 25.0))
  ;[0.1144 0.1144 0.1144] Call MovementController Move every Tick
  (`/Game/SuperMonkeyBall/Blueprint/AC_MovementController.Move` (`self.MovementController`) (`self.InputX`) (`self.InputY`) (`SceneComponent.GetRightVector` (`self.SpringArmRef`)))
  (`SceneComponent.K2_SetWorldRotation` _springarmref (`KismetMathLibrary.RInterpTo` (`SceneComponent.K2_GetComponentRotation` _springarmref) (`KismetMathLibrary.MakeRotator` (`KismetMathLibrary.Lerp` _roll (- _roll 10.0) (`self.InputX`)) (`KismetMathLibrary.Lerp` _returnvalue (+ _returnvalue 10.0) (`self.InputY`)) (.yaw (`KismetMathLibrary.Conv_VectorToRotator` (`/Game/SuperMonkeyBall/Blueprint/AC_MovementController.Velocity` (`self.MovementController`))))) (`GameplayStatics.GetWorldDeltaSeconds`) 1.0) false false))

(fn `GetCamera`
  (set `self.Camera` (`Actor.GetComponentByClass` (`self.GetOwner`) "/Script/Engine.CameraComponent")))