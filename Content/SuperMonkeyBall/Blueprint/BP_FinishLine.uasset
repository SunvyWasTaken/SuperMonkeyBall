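; BP_FinishLine is the goal trigger for the Super Monkey Ball game, switching to a rotating camera view when the monkey arrives.
; Overlap of its Box with a BP_Monkey blends the first player controller's view target to this actor.
; A looping timer at about 30 Hz then yaws the Scene component at a constant rate as a quick camera animation, without using Tick.
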(event `self.Box.OnComponentBeginOverlap`
  (params (OverlappedComponent :type "PrimitiveComponent Object Reference") (OtherActor :type "Actor Object Reference") (OtherComp :type "PrimitiveComponent Object Reference") (OtherBodyIndex :type Integer) (bFromSweep :type Boolean) (SweepResult :type "HitResult Structure (by ref)"))
  (cast `/Game/SuperMonkeyBall/Blueprint/BP_Monkey` OtherActor)
  (`PlayerController.SetViewTargetWithBlend` (`GameplayStatics.GetPlayerController` 0) self (`self.Blend Time`) "VTBlend_Linear" 0.0 false)
  ;[0.1144 0.1144 0.1144] Quick animation
  (`KismetSystemLibrary.K2_SetTimerDelegate` (delegate `RotateCamera`) 0.033333 true)
  (`self.RotateCamera`))

(event `RotateCamera`
  ;[0.1144 0.1144 0.1144] Quick animation
  (`SceneComponent.K2_AddLocalRotation` (`self.Scene`) (`KismetMathLibrary.MakeRotator` 0.0 0.0 (* 50.0 0.033333)) false false))

(fn `UserConstructionScript`)