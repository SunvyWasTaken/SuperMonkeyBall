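; Unfinished custom movement component for a Super Monkey Ball-style player, meant to move its owner by a Velocity vector.
; BeginPlay, Tick and both axis input functions are empty, with their logic left disconnected.
; The movement function adds normalized input or eases velocity toward zero as friction, but its inputs are zero.
; The gravity function, noted as not working, sphere-traces for ground with debug output, but its velocity corrections are unwired.
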(event `self.ReceiveTick`
  (params (DeltaSeconds :type "Float (single-precision)")))

(event `self.ReceiveBeginPlay`)

(fn `F_CalculeGravity`
  (locals (OutHit :type "HitResult Structure") (Radius :type "Float (single-precision)" :default 0.0))
  (bind _returnvalue (`self.GetOwner`))
  (bind _returnvalue_2 (`Actor.K2_GetActorLocation` (`self.GetOwner`)))
  (if (`self.IsActive`)
    (set `local.Radius` (`KismetMathLibrary.BreakVector3f` (`.BoxExtent` (`Actor.GetActorBounds` _returnvalue true false))))
    ;[1 1 1] POur le Debug
    (`KismetSystemLibrary.PrintString` (`KismetStringLibrary.Concat_StrStr` "Fall Velocity : " (`KismetStringLibrary.Conv_DoubleToString` 0.0)) true true (struct :`R` 1.0 :`G` 0.68913 :`A` 1.0) (`GameplayStatics.GetWorldDeltaSeconds`))
    (bind (_outhit _returnvalue_3) (`KismetSystemLibrary.SphereTraceSingle` :`Start` _returnvalue_2 :`End` (- (+ _returnvalue_2 (`self.Velocity`)) (+ (* (`Actor.GetActorUpVector` _returnvalue) -1.0 (0.0 0.0 0.0)) (0.0 0.0 25.0))) :`Radius` (`local.Radius`) :`TraceChannel` "TraceTypeQuery1" :`DrawDebugType` "ForOneFrame"))
    (set `local.OutHit` _outhit)
    (set `self.ISGrounded` (not _returnvalue_3))
    (if (`self.ISGrounded`)
      _)
    (else
      (return))))

(fn `F_CalculeMovement`
  (bind _returnvalue (`KismetMathLibrary.Normal` (+ (0.0 0.0 0.0) (0.0 0.0 0.0))))
  ;[0.8222 0 1] A revoir parce que jamais encore fait de truc avec la friction
  (if (<= (`KismetMathLibrary.VSize` _returnvalue) 0.0)
    (set `self.Velocity` (`KismetMathLibrary.VInterpTo_Constant` (`self.Velocity`) (0.0 0.0 0.0) (`GameplayStatics.GetWorldDeltaSeconds`) 50.0))
    (else
      (set `self.Velocity` (+ (`self.Velocity`) _returnvalue))))
  (return))

(fn `F_MoveForward`
  (params (Axis :type "Float (double-precision)")))

(fn `F_MoveRight`
  (params (Axis :type "Float (double-precision)")))