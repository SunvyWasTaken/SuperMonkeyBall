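; Game mode for Super Monkey Ball that runs the level countdown, the in-game HUD and the pause toggle.
; BeginPlay creates the interface widget and starts a looping one-second timer; GameTimer decrements the time down to zero and updates the HUD.
; FStopTimer clears that timer.
; FPause toggles game pause, the mouse cursor and the pause widget, which removes itself on resume.
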(event `self.ReceiveBeginPlay`
  ;[0.1144 0.1144 0.1144] Creation et affichage du widget, set des inputs sur le jeu.
  (`self.CreateWidgetInGame`)
  (`WidgetBlueprintLibrary.SetInputMode_GameOnly` (`GameplayStatics.GetPlayerController` 0))
  ;[0.1144 0.1144 0.1144] Active Le timer
  (bind _returnvalue (`KismetSystemLibrary.K2_SetTimerDelegate` (`|CreateDelegate` :!event `GameTimer`) 1.0 true))
  (set `self.TimerHandle` _returnvalue)
  (`self.GameTimer`))

(event `/Game/SuperMonkeyBall/Blueprint/BPI_Monkey.F_StopTimer`
  ;[0.1144 0.1144 0.1144] Clear the timer
  (`KismetSystemLibrary.K2_ClearAndInvalidateTimerHandle` (`self.TimerHandle`)))

(event `/Game/SuperMonkeyBall/Blueprint/BPI_Monkey.F_Pause`
  (if (`GameplayStatics.IsGamePaused`)
    (`GameplayStatics.SetGamePaused` false)
    (set `PlayerController.bShowMouseCursor` false (`GameplayStatics.GetPlayerController` 0))
    (bind _wpauseref (`self.WPauseRef`)
      (:`then`
        (`/Game/SuperMonkeyBall/Widget/WBP_Pause.F_SelfDestruct` _wpauseref))
      (:`else`))
    (else
      (`GameplayStatics.SetGamePaused` true)
      (bind _returnvalue (`|CreateWidget` "/Game/SuperMonkeyBall/Widget/WBP_Pause.WBP_Pause_C"))
      (set `self.WPauseRef` _returnvalue)
      (`UserWidget.AddToViewport` _returnvalue 0)
      (set `PlayerController.bShowMouseCursor` true (`GameplayStatics.GetPlayerController` 0)))))

(fn `CreateWidgetInGame`
  (bind _returnvalue (`|CreateWidget` "/Game/SuperMonkeyBall/Widget/WBP_Interface.WBP_Interface_C"))
  (set `self.InterfaceRef` _returnvalue)
  (`UserWidget.AddToViewport` _returnvalue 0))

(fn `GameTimer`
  (`self.InterfaceRef`
    (:`then`
      _)
    (:`else`
      (`self.CreateWidgetInGame`)))
  (if (not (<= (`self.CurrentTime`) 0))
    (`/Engine/EditorBlueprintResources/StandardMacros.DecrementInt` (`self.CurrentTime`)
      (:`  `
        (`/Game/SuperMonkeyBall/Widget/WBP_Interface.SetTimerText` (`self.InterfaceRef`) (`self.CurrentTime`))
        (return)))))

(fn `UserConstructionScript`)